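; BP_Pawn is a player pawn that slides sideways and spawns a BP_Ball, likely as the paddle in a ball game.
; Two handlers on one input axis offset the actor along Y in fixed, swept steps by the axis sign, without delta-time scaling.
; On BeginPlay, SpawnBall creates the ball at the Capsule's location, stores it in NewBall and binds to its OnDead event.
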(event `InputAxis|NewAxisMapping_0`
  (params (AxisValue :type "Float (single-precision)"))
  (if (< AxisValue 0.0)
    (`self.K2_AddActorWorldOffset` (0.0 -50.0 0.0) true)))

(event `InputAxis|NewAxisMapping_0`
  (params (AxisValue :type "Float (single-precision)"))
  (if (> AxisValue 0.0)
    (`self.K2_AddActorWorldOffset` (0.0 50.0 0.0) true)))

(event `self.ReceiveBeginPlay`
  (`self.SpawnBall`))

(fn `SpawnBall`
  (bind _returnvalue (`|SpawnActorFromClass` "/Game/Blueprints/BP_Ball.BP_Ball_C" (`KismetMathLibrary.MakeTransform` (`SceneComponent.K2_GetComponentLocation` (`self.Capsule`))) "AlwaysSpawn" "MultiplyWithRoot" null null))
  (bind _output_get (set `self.NewBall` _returnvalue))
  (add `/Game/Blueprints/BP_Ball.OnDead` _output_get (`|CreateDelegate` :!event `SpawnBall`))
  (return))

(fn `UserConstructionScript`)