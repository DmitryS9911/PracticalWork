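; BP_Decrease is an actor Blueprint that shrinks itself by 5% each time it registers a hit.
; Its Hit event calls the parent handler, scales the stored Size vector down, applies it as the actor's 3D scale and prints it on screen for debugging.
; The shrink compounds from the Size variable rather than the actor's current scale, with no minimum or filter on what it hits.
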(event `self.ReceiveHit`
  (params (MyComp :type "PrimitiveComponent Object Reference") (Other :type "Actor Object Reference") (OtherComp :type "PrimitiveComponent Object Reference") (bSelfMoved :type Boolean) (HitLocation :type "Vector Structure") (HitNormal :type "Vector Structure") (NormalImpulse :type "Vector Structure") (Hit :type "HitResult Structure (by ref)"))
  (`parent.ReceiveHit` MyComp Other OtherComp bSelfMoved HitLocation HitNormal NormalImpulse Hit)
  (bind _output_get (set `self.Size` (`self.Size`)))
  (bind _output_get_2 (set `self.Size` (* _output_get (0.95 0.95 0.95))))
  (`self.SetActorScale3D` _output_get_2)
  (`KismetSystemLibrary.PrintString` (`KismetStringLibrary.Conv_VectorToString` (`self.Size`)) true true (struct :`G` 0.66 :`B` 1.0 :`A` 1.0) 10.0))

(fn `UserConstructionScript`
  (`parent.UserConstructionScript`))