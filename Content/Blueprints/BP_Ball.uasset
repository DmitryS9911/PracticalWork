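; Ball actor that moves in a straight line and bounces off whatever blocks it, losing speed with each bounce.
; Tick moves it along Direction with a swept world offset, without physics simulation, and reflects Direction about the hit normal with Z zeroed.
; Each hit subtracts a fixed step, one tenth of the BeginPlay speed, down to MinSpeed, then prints the speed.
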(event `self.ReceiveBeginPlay`
  (set `self.Slowingdown` (* (`self.Speed`) 0.1)))

(event `self.ReceiveTick`
  (params (DeltaSeconds :type "Float (single-precision)"))
  (bind _sweephitresult (`self.K2_AddActorWorldOffset` (* (* (`self.Direction`) (`self.Speed`)) DeltaSeconds) true))
  (bind (_bblockinghit _binitialoverlap _time _distance _location _impactpoint _normal) (`GameplayStatics.BreakHitResult` _sweephitresult))
  (if _bblockinghit
    (bind (_returnvalue_x _returnvalue_y) (`KismetMathLibrary.BreakVector` (`KismetMathLibrary.GetReflectionVector` (`self.Direction`) _normal)))
    (set `self.Direction` (`KismetMathLibrary.MakeVector` _returnvalue_x _returnvalue_y))
    (bind _output_get (set `self.Speed` (`KismetMathLibrary.FMax` (- (`self.Speed`) (`self.Slowingdown`)) (`self.MinSpeed`))))
    (`KismetSystemLibrary.PrintString` (`KismetStringLibrary.Conv_DoubleToString` _output_get))))

(fn `UserConstructionScript`)